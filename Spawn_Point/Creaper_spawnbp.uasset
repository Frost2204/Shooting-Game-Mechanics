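; Creeper spawn point Blueprint that, on BeginPlay, spawns a set number of actors at random locations inside its Bound component's box.
; Each spawn picks a random point in the bounds and a yaw from RandomFloat, which only ranges from 0 to 1 degree.
; A debug-drawn downward-offset WorldStatic line trace runs first, but its result is unused, so spawns are not snapped to ground.
; The spawned class is set to base Actor.
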(event `self.ReceiveBeginPlay`
  (for _ (range 1 (+ (`self.Spawn Amount`) 1))
    (`self.spawn_character`)))

(fn `spawn_character`
  (bind (_origin _boxextent) (`KismetSystemLibrary.GetComponentBounds` (`self.bound`)))
  (bind _returnvalue (`KismetMathLibrary.RandomPointInBoundingBox` _origin _boxextent))
  (bind _outhit (`KismetSystemLibrary.LineTraceSingleForObjects` :`End` (+ (`KismetMathLibrary.MakeVector` (.x _returnvalue) (.y _returnvalue) (+ (.z _returnvalue) 10000.0)) (* (* (`self.GetActorUpVector`) -1.0) 15000.0)) :`ObjectTypes` (`|MakeArray` "ObjectTypeQuery1" :!type "EObjectTypeQuery Enum") :`DrawDebugType` "ForDuration"))
  (`|SpawnActorFromClass` "/Script/Engine.Actor" (`KismetMathLibrary.MakeTransform` _returnvalue (`KismetMathLibrary.MakeRotator` 0.0 0.0 (`KismetMathLibrary.RandomFloat`))) "Undefined" "OverrideRootScale" null null))

(fn `UserConstructionScript`)